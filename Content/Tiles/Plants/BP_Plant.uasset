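; BP_Plant is a plant tile actor with a configurable mesh, health, production and range, plus a details widget created at BeginPlay.
; It starts at zero scale; Grow briefly opens a Tick gate that spring-interpolates the mesh toward a scale derived from its stats.
; Damage draws a debug arrow from the cause and plays a wiggle timeline, adding a shrink-then-destroy timeline when lethal.
; Production changes fire a notification call.
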(event EventOnDamageRecived
  (params (Amount :type Integer) (Cause :type Tile%20Object%20Reference) (bShouldDestroy :type Boolean))
  (Variables|Hidden|SetDead bShouldDestroy)
  (Rendering|Debug|DrawDebugArrow (+ (Transformation|GetActorLocation Cause) "0.000000,0,1.000000") (+ (Transformation|GetActorLocation) "0,0,1.000000") 5e+01 "(R=0.219226,G=0.000000,B=0.404167,A=1.000000)" 4.0 5.0)
  (if (Variables|Hidden|GetDead)
    (Utilities|FlowControl|Sequence
      (:then_0
        ;[1 1 1] Shrink
        (bind _scale (Timeline|Die Play)
          (:Update
            (Transformation|SetRelativeScale3D (Variables|Default|GetPlantMesh) (Math|Conversions|ToVector(Float) (* (CallFunction|GetTargetScale) _scale))))
          (:Finished
            (Actor|DestroyActor))))
      (:then_1
        ;[1 1 1] Shake
        (bind _rotation (Timeline|Wiggle PlayFromStart)
          (:Update
            (Transformation|SetRelativeRotation (Variables|Default|GetPlantMesh) (Math|Rotator|MakeRotator (.x _rotation) (.y _rotation) 0.0) false false)))))
    (else
      (Timeline|Wiggle PlayFromStart))))

(event EventBeginPlay
  (|CallParentFunction)
  (Transformation|SetRelativeScale3D (Variables|Default|GetPlantMesh) "0, 0, 0")
  (bind _returnvalue (UserInterface|CreateWidget "/Game/UI/Details/WBP_PlantDetails.WBP_PlantDetails_C" 0 self))
  (Variables|Hidden|SetDetailsWidget _returnvalue))

(event EventGrow
  (if (not (Variables|Hidden|GetDead))
    (|CallParentFunction)
    (Utilities|FlowControl|Sequence
      (:then_0
        (Utilities|FlowControl|Delay 2.0)
        ;[1 1 1] Get Bigger
        (Utilities|FlowControl|Gate true) ; enters at Close
      )
      (:then_1
        (Utilities|FlowControl|Gate true) ; enters at Open
      ))
    (else
      (|CallParentFunction))))

(event EventTick
  (params (DeltaSeconds :type Float%20%28single-precision%29))
  ;[1 1 1] Get Bigger
  (Utilities|FlowControl|Gate true
    (:Exit
      (bind _returnvalue (Class|KismetMathLibrary|FloatSpringInterp (.x (Variables|/Script/Engine.SceneComponent|GetRelativeScale3D (Variables|Default|GetPlantMesh))) (CallFunction|GetTargetScale) (Variables|Hidden|GetGrowSpringState) 1e+02 0.3 DeltaSeconds 1.0 1.0))
      (Transformation|SetRelativeScale3D (Variables|Default|GetPlantMesh) (Math|Conversions|ToVector(Float) _returnvalue)))))

(event EventSetProduction
  (params (NewProduction :type Integer))
  (|CallParentFunction NewProduction)
  (Default|CallProductionChanged))

(fn ConstructionScript
  (Components|StaticMesh|SetStaticMesh (Variables|Default|GetPlantMesh) (Variables|Visuals|GetMesh)))

(fn GetTargetScale
  (return (/ (Math|Conversions|ToFloat(Integer) (+ (Class|Plant|GetHealth) (Class|Plant|GetProduction) (Class|Plant|GetRange))) (+ 0 0 0))))

(fn GetMaxPlantSize
  (return 0))