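; Tile obstacle that works out which grid subtiles its mesh covers whenever its construction script runs.
; It temporarily moves the mesh near the world origin and sizes a padded grid from its rotated, scaled bounds.
; A vertical component sphere trace at each cell records hits in RelativeSubTileLocations as offsets from the grid centre.
; Afterwards it restores the mesh to relative placement on the actor, undoing the grid-height alignment shift.
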(fn ConstructionScript
  (CallFunction|UpdateSubtileLocations))

(fn UpdateSubtileLocations
  (bind _returnvalue (Class|GridLibrary|GetGridHeight))
  (bind _returnvalue_2 (Class|GridLibrary|GetGridHeight))
  (bind _meshcomponent (Variables|Default|GetMeshComponent))
  (bind _meshcomponent_2 (Variables|Default|GetMeshComponent))
  (bind _meshcomponent_3 (Variables|Default|GetMeshComponent))
  (bind (_min _max) (Components|StaticMesh|GetLocalBounds _meshcomponent))
  (bind _returnvalue_3 (Transformation|GetWorldTransform _meshcomponent_2))
  (bind _returnvalue_4 (* _returnvalue 0.333333))
  (bind _returnvalue_5 (Math|Vector|VectorGetAbs _min))
  (bind _returnvalue_6 (Math|Vector|VectorGetAbs _max))
  (bind _returnvalue_7 (Math|Transform|MakeTransform "0, 0, 0" (.rotation _returnvalue_3) (.scale _returnvalue_3)))
  (bind _returnvalue_8 (Math|Vector|VectorComponentMax _returnvalue_5 _returnvalue_6))
  (bind _returnvalue_9 (Math|Transform|TransformLocation _returnvalue_7 _returnvalue_8))
  (bind _returnvalue_10 (* _returnvalue_8 "-1.000000,1.000000,0"))
  (bind _returnvalue_11 (Math|Vector|VectorGetAbs _returnvalue_9))
  (bind _returnvalue_12 (Math|Transform|TransformLocation _returnvalue_7 _returnvalue_10))
  (bind _returnvalue_13 (Math|Vector|VectorGetAbs _returnvalue_12))
  (bind _returnvalue_14 (Math|Vector|VectorComponentMax _returnvalue_11 _returnvalue_13))
  (bind _returnvalue_15 (* _returnvalue_14 2.0))
  (bind _returnvalue_16 (Class|GridLibrary|WorldLocationtoGridLocation _returnvalue_15))
  (bind _returnvalue_17 (+ _returnvalue_16 (Utilities|Struct|MakeIntPoint 4 4)))
  (Components|StaticMesh|SetStaticMesh (Variables|Default|GetMeshComponent) (Variables|Mesh|GetMesh))
  ;[1 1 1] Move Mesh To Orgin
  (Transformation|SetWorldTransform (Variables|Default|GetMeshComponent) (Math|Transform|ComposeTransforms (Variables|Mesh|GetMeshTransform) (Math|Transform|MakeTransform (Math|Vector|MakeVector _returnvalue_4 0.0 0.0))) false false)
  (Utilities|FlowControl|Sequence
    (:then_0
      (Utilities|Set|Clear (Variables|Default|GetRelativeSubTileLocations))
      (bind (_current_point _total_points _0_1_phase _poly_center _x_row _y_row) (Utilities|2DGridExecutionMacro :Sector%20Size 1.0 :X (.x _returnvalue_17) :Y (.y _returnvalue_17))
        (:Per%20Poly%20Execution
          ;[1 1 1] Trace each tile for overlap with the mesh
          (bind _returnvalue_18 (Class|PrimitiveComponent|SphereTraceComponent (Variables|Default|GetMeshComponent) (+ (* (+ (+ (Class|GridLibrary|GridLocationtoWorldLocation (Utilities|Operators|Subtract (Utilities|Struct|MakeIntPoint _x_row _y_row) (Utilities|Struct|MakeIntPoint 2 2) (/ _returnvalue_16 (Utilities|Struct|MakeIntPoint 2 2)))) (Math|Vector|MakeVector (* _returnvalue_2 -0.666666) 0.0 0.0)) (Math|Vector|MakeVector (* _returnvalue_2 0.5) 0.0 0.0)) "1.000000,1.000000,0") "0,0,500.000000") (* (+ (+ (Class|GridLibrary|GridLocationtoWorldLocation (Utilities|Operators|Subtract (Utilities|Struct|MakeIntPoint _x_row _y_row) (Utilities|Struct|MakeIntPoint 2 2) (/ _returnvalue_16 (Utilities|Struct|MakeIntPoint 2 2)))) (Math|Vector|MakeVector (* _returnvalue_2 -0.666666) 0.0 0.0)) (Math|Vector|MakeVector (* _returnvalue_2 0.5) 0.0 0.0)) "1.000000,1.000000,0") (/ (Class|GridLibrary|GetGridSideLength) 1.5) true false true))
          (if _returnvalue_18
            (Utilities|Set|Add (Variables|Default|GetRelativeSubTileLocations) (Utilities|Operators|Subtract (Utilities|Struct|MakeIntPoint _x_row _y_row) (Utilities|Struct|MakeIntPoint 2 2) (/ _returnvalue_16 (Utilities|Struct|MakeIntPoint 2 2))))))))
    (:then_1
      (Transformation|SetRelativeTransform _meshcomponent_3 (Math|Transform|ComposeTransforms (Transformation|GetWorldTransform _meshcomponent_3) (Math|Transform|MakeTransform (Math|Vector|MakeVector (* _returnvalue_4 -1.0) 0.0 0.0))) false false)
      (Transformation|SetAbsolute _meshcomponent_3 false false false))))