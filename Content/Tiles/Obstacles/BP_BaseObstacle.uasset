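; Base obstacle tile Blueprint that computes which grid subtiles its mesh covers, rebuilt in the construction script.
; It temporarily places the mesh at its relative transform in world space, so the resulting cells are actor-relative.
; It line-traces downward against the mesh over a padded bounds grid, storing hit cells in RelativeSubTileLocations.
; Persistent debug traces and points visualize the result, then the mesh transform is restored.
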(fn ConstructionScript
  (CallFunction|UpdateSubtileLocations))

(fn UpdateSubtileLocations
  (bind _returnvalue (Class|GridLibrary|GetGridHeight))
  (bind _mesh (Variables|Default|GetMesh))
  (bind _mesh_2 (Variables|Default|GetMesh))
  (bind _mesh_3 (Variables|Default|GetMesh))
  (bind _mesh_4 (Variables|Default|GetMesh))
  (bind (_min _max) (Components|StaticMesh|GetLocalBounds _mesh))
  (bind _returnvalue_2 (Transformation|GetWorldTransform _mesh_3))
  (bind _returnvalue_3 (Math|Transform|TransformLocation _returnvalue_2 _max))
  (bind _returnvalue_4 (Math|Transform|TransformLocation _returnvalue_2 _min))
  (bind _returnvalue_5 (Math|Vector|VectorComponentMin _returnvalue_4 _returnvalue_3))
  (bind _returnvalue_6 (Math|Vector|VectorComponentMax _returnvalue_4 _returnvalue_3))
  (bind _returnvalue_7 (Class|GridLibrary|WorldLocationtoGridLocation _returnvalue_6))
  (bind _returnvalue_8 (Class|GridLibrary|WorldLocationtoGridLocation _returnvalue_5))
  (bind _returnvalue_9 (Utilities|Operators|Subtract _returnvalue_7 _returnvalue_8 (Utilities|Struct|MakeIntPoint -3 -3)))
  (Transformation|SetWorldTransform _mesh_2 (Transformation|GetRelativeTransform _mesh_2) false false)
  (Utilities|FlowControl|Sequence
    (:then_0
      (Utilities|Set|Clear (Variables|Default|GetRelativeSubTileLocations))
      (Rendering|Debug|FlushPersistentDebugLines)
      (bind (_current_point _total_points _0_1_phase _poly_center _x_row _y_row) (Utilities|2DGridExecutionMacro :Sector%20Size 1.0 :X (.x _returnvalue_9) :Y (.y _returnvalue_9))
        (:Per%20Poly%20Execution
          (bind (_hitlocation _hitnormal _bonename _outhit _returnvalue_10) (Collision|LineTraceComponent (Variables|Default|GetMesh) (+ (* (+ (+ (Class|GridLibrary|GridLocationtoWorldLocation (+ (Utilities|Struct|MakeIntPoint _x_row _y_row) _returnvalue_8 (Utilities|Struct|MakeIntPoint -1 -1))) (Math|Vector|MakeVector (* _returnvalue -0.666666) 0.0 0.0)) (Math|Vector|MakeVector (* _returnvalue 0.5) 0.0 0.0)) "1.000000,1.000000,0") "0,0,500.000000") (* (+ (+ (Class|GridLibrary|GridLocationtoWorldLocation (+ (Utilities|Struct|MakeIntPoint _x_row _y_row) _returnvalue_8 (Utilities|Struct|MakeIntPoint -1 -1))) (Math|Vector|MakeVector (* _returnvalue -0.666666) 0.0 0.0)) (Math|Vector|MakeVector (* _returnvalue 0.5) 0.0 0.0)) "1.000000,1.000000,0") true true true))
          (if _returnvalue_10
            (Rendering|Debug|DrawDebugPoint _hitlocation 2e+01 "(R=0.116303,G=0.089244,B=0.641667,A=1.000000)" 321213.0)
            (Utilities|Set|Add (Variables|Default|GetRelativeSubTileLocations) (+ (Utilities|Struct|MakeIntPoint _x_row _y_row) _returnvalue_8 (Utilities|Struct|MakeIntPoint -1 -1)))))))
    (:then_1
      (Transformation|SetRelativeTransform _mesh_4 (Transformation|GetWorldTransform _mesh_4) false false)
      (Transformation|SetAbsolute _mesh_4 false false false))))