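; BP_RangePreviewer is an instanced mesh component that displays a tile range preview around a given grid shape.
; UpdatePreview grows the shape by the range with ScaleShapeUp, then converts each resulting grid location to a transform with an Up direction.
; It reuses existing instances, adds missing ones and runs a removal loop for surplus ones, flagging render state dirty only when updating the last existing instance.
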(event Custom|UpdatePreview
  (params (InitialShape :type Set%20of%20Int%20Point%20Structures) (Range :type Integer))
  (bind _returnvalue (Components|InstancedStaticMesh|GetInstanceCount))
  (bind _result (Utilities|Set|ToArray (Class|GridLibrary|ScaleShapeUp InitialShape Range false)))
  (for (_array_element _array_index) _result
    (if (>= _array_index _returnvalue)
      (Components|InstancedStaticMesh|AddInstance (Class|GridLibrary|GridTransformtoWorldTransform (Utilities|Struct|MakeGridTransform _array_element "Up")) false)
      (else
        (Components|InstancedStaticMesh|UpdateInstanceTransform _array_index (Class|GridLibrary|GridTransformtoWorldTransform (Utilities|Struct|MakeGridTransform _array_element "Up")) false (== _array_index (- _returnvalue 1)) false))))
  (for _index (range (Utilities|Array|Length _result) (- _returnvalue 1))
    (Class|InstancedStaticMeshComponent|RemoveInstance _index)))