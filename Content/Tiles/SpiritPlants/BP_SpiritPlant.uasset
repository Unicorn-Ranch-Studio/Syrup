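; Spirit plant tile that displays a glowing version of its PlantClass and applies field and trash-spawn-blocking effects around itself.
; The construction script copies the plant's mesh and one-step-expanded sub-tile footprint, centers the mesh on that footprint's grid bounds and applies a glow material.
; BeginPlay creates its details widget and activates both effects over its sub-tiles, again expanded by one step.
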(event EventBeginPlay
  (|CallParentFunction)
  (bind _returnvalue (UserInterface|CreateWidget "/Game/UI/Details/WBP_SpiritPlantDetails.WBP_SpiritPlantDetails_C" 0 self))
  (bind _output_get (Variables|Default|SetDetailsWidget _returnvalue))
  (Default|SetSpiritPlant _output_get self)
  (Class|TileEffect|ActivateEffect (Variables|Default|GetApplyField) "OnActivated" 0 (Class|GridLibrary|ScaleShapeUp (Class|Tile|GetSubTileLocations) 1 false)))

(fn ConstructionScript
  (bind _returnvalue (Class|GridLibrary|GetGridHeight))
  (bind _returnvalue_2 (Class|GridLibrary|GetGridSideLength))
  (bind _returnvalue_3 (/ _returnvalue_2 2.0))
  (bind _returnvalue_4 (Math|Vector|MakeVector _returnvalue _returnvalue_3 0.0))
  (Utilities|Set|Clear (Variables|Default|GetRelativeSubTileLocations))
  (bind _result (Utilities|Set|ToArray (Class|GridLibrary|ScaleShapeUp (.RelativeSubTileLocations (Utilities|GetClassDefaults (Variables|Default|GetPlantClass))) 1 false)))
  (for _array_element _result
    (Utilities|Set|Add (Variables|Default|GetRelativeSubTileLocations) _array_element)
    (LocalVariables|SetMin (Utilities|Struct|MakeIntPoint (Math|Integer|Min(Integer) (.x (LocalVariables|GetMin)) (.X (Utilities|Struct|BreakIntPoint _array_element))) (Math|Integer|Min(Integer) (.y (LocalVariables|GetMin)) (.Y (Utilities|Struct|BreakIntPoint _array_element)))))
    (LocalVariables|SetMax (Utilities|Struct|MakeIntPoint (Math|Integer|Max(Integer) (.x (LocalVariables|GetMax)) (.X (Utilities|Struct|BreakIntPoint _array_element))) (Math|Integer|Max(Integer) (.Y (Utilities|Struct|BreakIntPoint _array_element)) (.y (LocalVariables|GetMax))))))
  (Components|StaticMesh|SetStaticMesh (Variables|Default|GetMesh) (.Mesh (Utilities|GetClassDefaults (Variables|Default|GetPlantClass))))
  (Transformation|SetRelativeLocation (Variables|Default|GetMeshRoot) (- (* (Math|Vector|GetVectorArrayAverage (Utilities|Array|MakeArray (* (+ (Math|Conversions|ToVector(Vector2D) (Math|Conversions|ToVector2D(IntPoint) (LocalVariables|GetMin))) "0,-1.000000,0") _returnvalue_4) (* (+ (Math|Conversions|ToVector(Vector2D) (Math|Conversions|ToVector2D(IntPoint) (LocalVariables|GetMax))) "1.000000,1.000000,0") _returnvalue_4))) "1.000000,1.000000,0") (Math|Vector|MakeVector (* (Class|GridLibrary|GetGridHeight) 0.333333) 0.0 0.0)) false false)
  (for _index (range 0 (- (Rendering|Material|GetNumMaterials (Variables|Default|GetMesh)) 1))
    (Rendering|Material|SetMaterial (Variables|Default|GetMesh) _index "/Game/ColorPallet/Matierals/Plants/M_Plant_Glow.M_Plant_Glow")))