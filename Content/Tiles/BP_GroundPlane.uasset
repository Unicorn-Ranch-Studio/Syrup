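; BP_GroundPlane is a tile actor that builds a grid-aligned ground plane from instanced static meshes, sized by its Size variable.
; The construction script clears existing instances, then runs a 2D grid macro that converts each cell to a world transform composed with a small downward Z offset.
; It adds all collected transforms in one batched world-space call.
; The event graph has no active logic.
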(event EventBeginPlay)

(event Collision|EventActorBeginOverlap
  (params (OtherActor :type Actor%20Object%20Reference)))

(event EventTick
  (params (DeltaSeconds :type Float%20%28single-precision%29)))

(fn ConstructionScript
  (bind _size (Variables|Default|GetSize))
  (Components|InstancedStaticMesh|ClearInstances (Variables|Default|GetInstancedStaticMesh))
  (Utilities|FlowControl|Sequence
    (:then_0
      (bind _poly_center (Utilities|2DGridExecutionMacro :Sector%20Size 1.0 :X (.x _size) :Y (.y _size))
        (:Per%20Poly%20Execution
          (Utilities|Array|Add (LocalVariables|GetInstanceTransforms) (Math|Transform|ComposeTransforms (Class|GridLibrary|GridLocationtoWorldTransform (Class|KismetMathLibrary|ToIntPoint(Vector2D) (Math|Conversions|ToVector2D(Vector) _poly_center))) (Math|Transform|MakeTransform "0, 0,-1.000000" "0, 0, 0" "1.000000,1.000000,1.000000"))))))
    (:then_1
      (Components|InstancedStaticMesh|AddInstances (Variables|Default|GetInstancedStaticMesh) (LocalVariables|GetInstanceTransforms) false true))))