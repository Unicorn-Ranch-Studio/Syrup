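; BP_Trash is a trash prop, filed under tiles, that drops into place when play begins.
; On BeginPlay it moves TrashMesh to FallFromLocation, waits a random delay of up to a second, then a timeline lerps it back to its original relative location.
; Landing plays a world camera shake at the actor and calls OnFinishedFalling; the branch that skips the fall is disabled by a hard-coded true.
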(event EventBeginPlay
  (bind _trashmesh (Variables|Default|GetTrashMesh))
  (if true
    (Variables|Default|SetRelativeMeshLocation (Variables|/Script/Engine.SceneComponent|GetRelativeLocation _trashmesh))
    (Transformation|SetRelativeLocation _trashmesh (Variables|Default|GetFallFromLocation) false false)
    (Utilities|FlowControl|Delay (Math|Random|RandomFloat))
    (bind _percentfallen (Timeline|Fall Play)
      (:Update
        (Transformation|SetRelativeLocation (Variables|Default|GetTrashMesh) (Math|Vector|Lerp(Vector) (Variables|Default|GetFallFromLocation) (Variables|Default|GetRelativeMeshLocation) _percentfallen) false false))
      (:Finished
        (Camera|PlayWorldCameraShake "/Game/Tiles/Trash/BP_Trash_LandedShake.BP_Trash_LandedShake_C" (Transformation|GetActorLocation) 0.0 2e+03)
        (Class|Trash|OnFinishedFalling)))
    (else
      (Class|Trash|OnFinishedFalling))))

(fn ConstructionScript
  (|CallParentFunction))