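; BP_Pesticides is a pesticide trash tile that switches on three effect components, likely Niagara systems, once it has landed.
; It extends the parent's fall-finished event to activate NSPesticides, NSPesticides1 and NSPesticides2 without resetting them.
; BeginPlay triggers the same activation when game time is exactly zero, so tiles present at game start show the effects without waiting for a fall.
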(event EventBeginPlay
  (|CallParentFunction)
  (if (== (Utilities|Time|GetGameTimeinSeconds) 0.0)
    (Components|Activation|Activate (Variables|Default|GetNS_Pesticides) false)))

(event EventFallFinishedFunc
  (|CallParentFunction)
  (Components|Activation|Activate (Variables|Default|GetNS_Pesticides) false))

(fn ConstructionScript
  (|CallParentFunction))