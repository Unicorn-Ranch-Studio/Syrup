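; Game mode that runs the repeating turn cycle for a tile-based game of plants and spreading trash.
; Every few seconds it restarts the Night timeline, which drives the directional light's intensity, and broadcasts PlantsGrow when that finishes.
; The plant-active and trash damage, active and spread triggers fire in order as the timeline starts, without waiting for it.
; All triggers pass empty location sets through the tile-effect delegate.
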(event EventBeginPlay
  (bind _set (Utilities|Set|MakeSet))
  (bind _returnvalue (Actor|GetActorOfClass "/Script/Engine.DirectionalLight"))
  (Utilities|FlowControl|Delay 5.0 :!label _label)
  (Utilities|FlowControl|Sequence
    (:then_0
      (bind _intensity (Timeline|Night PlayFromStart)
        (:Update
          (Rendering|Components|Light|SetIntensity (Variables|/Script/Engine.Light|GetLightComponent _returnvalue) _intensity))
        (:Finished
          (Default|CallTileEffectTriggerDelegate "PlantsGrow" _set))))
    (:then_1
      (Default|CallTileEffectTriggerDelegate "PlantActive" _set)
      (Default|CallTileEffectTriggerDelegate "TrashDamage" _set)
      (Default|CallTileEffectTriggerDelegate "TrashActive" _set)
      (Default|CallTileEffectTriggerDelegate "TrashSpread" _set)
      (goto _label))))

(fn ConstructionScript)