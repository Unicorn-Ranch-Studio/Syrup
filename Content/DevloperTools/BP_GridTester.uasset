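; Developer test actor that probes the game's grid at its own location in the editor.
; Its Construction Script snaps the actor location to a grid cell, runs OverlapGridLocation and draws a short-lived debug point colored by the result.
; Disconnected experiments visualize direction-transformed tile shapes over a grid area.
; An uncalled helper, DrawDebugTriangle, outlines a rotated triangle from grid height and side length.
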(event EventBeginPlay)

(event Collision|EventActorBeginOverlap
  (params (OtherActor :type Actor%20Object%20Reference)))

(event EventTick
  (params (DeltaSeconds :type Float%20%28single-precision%29)))

(fn ConstructionScript
  (bind _returnvalue (Transformation|GetActorLocation))
  (bind _returnvalue_2 (Class|GridLibrary|WorldLocationtoGridLocation _returnvalue))
  (bind _returnvalue_3 (Class|GridLibrary|OverlapGridLocation _returnvalue_2))
  (Rendering|Debug|DrawDebugPoint (.location (Class|GridLibrary|GridLocationtoWorldTransform _returnvalue_2)) 2e+01 (select _returnvalue_3 "(R=1.000000,G=0.000000,B=0.936766,A=1.000000)" "") 5.0))

(fn DrawDebugTriangle
  (params (Location :type Vector) (Rotation :type Rotator) (LineColor :type Linear%20Color%20Structure) (Duration :type Float%20%28single-precision%29) (Thickness :type Float%20%28single-precision%29))
  (bind _returnvalue (Class|GridLibrary|GetGridSideLength))
  (bind _returnvalue_2 (Class|GridLibrary|GetGridHeight))
  (bind _returnvalue_3 (Class|GridLibrary|GetGridSideLength))
  (bind _returnvalue_4 (Class|GridLibrary|GetGridHeight))
  (bind _returnvalue_5 (Class|GridLibrary|GetGridHeight))
  (bind _returnvalue_6 (* _returnvalue_5 -0.333333))
  (bind _returnvalue_7 (* _returnvalue_2 -0.333333))
  (bind _returnvalue_8 (* _returnvalue_3 0.5))
  (bind _returnvalue_9 (* _returnvalue_4 0.666667))
  (bind _returnvalue_10 (* _returnvalue -0.5))
  (bind _returnvalue_11 (Math|Vector|RotateVector (Math|Vector|MakeVector _returnvalue_6 _returnvalue_10 0.0) Rotation))
  (bind _returnvalue_12 (Math|Vector|RotateVector (Math|Vector|MakeVector _returnvalue_9 0.0 0.0) Rotation))
  (bind _returnvalue_13 (Math|Vector|RotateVector (Math|Vector|MakeVector _returnvalue_7 _returnvalue_8 0.0) Rotation))
  (bind _returnvalue_14 (+ Location _returnvalue_13))
  (bind _returnvalue_15 (+ Location _returnvalue_11))
  (bind _returnvalue_16 (+ Location _returnvalue_12))
  (Rendering|Debug|DrawDebugLine _returnvalue_16 _returnvalue_14 LineColor Duration Thickness)
  (Rendering|Debug|DrawDebugLine _returnvalue_16 _returnvalue_15 LineColor Duration Thickness)
  (Rendering|Debug|DrawDebugLine _returnvalue_14 _returnvalue_15 LineColor Duration Thickness))