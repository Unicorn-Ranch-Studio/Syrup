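; BP_TestNPC is a test NPC that shows a dialogue box when the player interacts with it nearby.
; Sphere overlap with BP_SyrupPlayerCharacter binds and unbinds the Stoopid event to that character's interact input.
; Stoopid creates a WBP_DialogueBox with the NPC's Dialogue text, unless one already exists.
; Leaving the sphere removes the widget and clears its reference, allowing a fresh box next time.
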(event OnComponentBeginOverlap(Sphere1)
  (params (OverlappedComponent :type Primitive%20Component%20Object%20Reference) (OtherActor :type Actor%20Object%20Reference) (OtherComp :type Primitive%20Component%20Object%20Reference) (OtherBodyIndex :type Integer) (bFromSweep :type Boolean) (SweepResult :type Hit%20Result%20Structure%20%28by%20ref%29))
  (bind _asbp_syrup_player_character (Utilities|Casting|CastToBP_SyrupPlayerCharacter OtherActor))
  (EventDispatchers|BindEventtoInteract _asbp_syrup_player_character (delegate Custom|Stoopid)))

(event OnComponentEndOverlap(Sphere1)
  (params (OverlappedComponent :type Primitive%20Component%20Object%20Reference) (OtherActor :type Actor%20Object%20Reference) (OtherComp :type Primitive%20Component%20Object%20Reference) (OtherBodyIndex :type Integer))
  (bind _asbp_syrup_player_character (Utilities|Casting|CastToBP_SyrupPlayerCharacter OtherActor))
  (EventDispatchers|UnbindEventfromInteract _asbp_syrup_player_character (delegate Custom|Stoopid))
  (Utilities|IsValid (Variables|Default|GetCreatedDialogueWidget)
    (:Is%20Valid
      (Widget|RemovefromParent (stale Custom|Stoopid _returnvalue))
      (Variables|Default|SetCreatedDialogueWidget 0))))

(event Custom|Stoopid
  (Utilities|IsValid (Variables|Default|GetCreatedDialogueWidget)
    (:Is%20Not%20Valid
      (bind _returnvalue (UserInterface|CreateWidget "/Game/UI/WBP_DialogueBox.WBP_DialogueBox_C"))
      (Variables|Default|SetCreatedDialogueWidget _returnvalue)
      (Variables|/Game/UI/WBP_DialogueBox.WBP_DialogueBox_C|SetCurrentDialogue _returnvalue (Utilities|Text|ToText(String) (Variables|Default|GetDialogue)))
      (UserInterface|Viewport|AddtoViewport _returnvalue 0))))

(fn ConstructionScript)