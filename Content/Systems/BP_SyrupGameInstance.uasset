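; Game instance that manages rotating, timestamp-named autosave slots, indexed in a persistent SavesList save object loaded or created on Init.
; SaveAutosave replaces the slot after the newest, wrapping at MaxAutosaves, and ClearAutosaves deletes all.
; LoadAutosave reopens L_Test and re-arms a DoOnce, so the next LevelOpened loads the newest autosave.
; The first LevelOpened triggers LoadAutosave itself, so startup restores via a level reopen.
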(event Custom|LoadAutosave
  (bind (_returnvalue _savetime) (CallFunction|GetMostRecentAutosave))
  (Game|OpenLevel(byObjectReference) "/Game/Levels/L_Test.L_Test")
  (Utilities|FlowControl|DoOnce true) ; enters at Reset
)

(event Custom|LevelOpened
  (bind (_returnvalue _savetime) (CallFunction|GetMostRecentAutosave))
  (Utilities|FlowControl|Sequence
    (:then_0
      (Utilities|FlowControl|DoOnce true
        (:Completed
          (if _returnvalue
            (Class|SyrupSaveGame|LoadGame (CallFunction|GetSaveSlotName _savetime))))))
    (:then_1
      (Utilities|FlowControl|DoOnce false
        (:Completed
          (CallFunction|LoadAutosave))))))

(event EventInit
  (bind _returnvalue (SaveGame|LoadGamefromSlot (Variables|Default|GetSaveListSlot)))
  (bind _asbp_saves_list_save (Utilities|Casting|CastToBP_SavesListSave _returnvalue)
    (:then
      (Variables|Default|SetSavesList _asbp_saves_list_save))
    (:CastFailed
      (bind _returnvalue_2 (SaveGame|CreateSaveGameObject "/Game/Systems/BP_SavesListSave.BP_SavesListSave_C"))
      (Variables|Default|SetSavesList _returnvalue_2))))

(fn GetMostRecentAutosave
  (bind _saveslist (Variables|Default|GetSavesList)
    (:then
      (for (_array_element _array_index) (Variables|/Game/Systems/BP_SavesListSave.BP_SavesListSave_C|GetAutosaves _saveslist)
        (if (> _array_element (LocalVariables|GetMostRecentTime))
          (LocalVariables|SetMostRecentTime _array_element)
          (LocalVariables|SetMostRecentIndex _array_index)))
      (if (Utilities|Array|IsNotEmpty (Variables|/Game/Systems/BP_SavesListSave.BP_SavesListSave_C|GetAutosaves _saveslist))
        (return true (LocalVariables|GetMostRecentTime) (LocalVariables|GetMostRecentIndex))
        (else
          (return false "" -1))))
    (:else
      (return false "" -1))))

(fn GetSaveSlotName
  (params (SaveDateTime :type Date%20Time%20Structure))
  (bind (_year _month _day _hour _minute _second) (Math|DateTime|BreakDateTime SaveDateTime))
  (return (Utilities|String|ToString(Text) (Utilities|Text|FormatText "Autosave_{Hour}-{Minute}-{Second}_{Day}-{Month}-{Year}" _hour _minute _day _month (Utilities|String|ToString(Integer) _year) _second))))

(fn SaveAutosave
  (LocalVariables|SetSaveIndex (Math|Integer|%(Integer) (+ (.Index (CallFunction|GetMostRecentAutosave)) 1) (Variables|Default|GetMaxAutosaves)))
  (if (Utilities|Array|IsValidIndex (Variables|/Game/Systems/BP_SavesListSave.BP_SavesListSave_C|GetAutosaves (Variables|Default|GetSavesList)) (LocalVariables|GetSaveIndex))
    (SaveGame|DeleteGameinSlot (CallFunction|GetSaveSlotName (Utilities|Array|Get(acopy) (Variables|/Game/Systems/BP_SavesListSave.BP_SavesListSave_C|GetAutosaves (Variables|Default|GetSavesList)) (LocalVariables|GetSaveIndex)))))
  (bind _output_get (LocalVariables|SetSaveTime (Math|DateTime|Now)))
  (Class|SyrupSaveGame|SaveGame (CallFunction|GetSaveSlotName _output_get))
  (Utilities|Array|SetArrayElem (Variables|/Game/Systems/BP_SavesListSave.BP_SavesListSave_C|GetAutosaves (Variables|Default|GetSavesList)) (LocalVariables|GetSaveIndex) (LocalVariables|GetSaveTime) true)
  (SaveGame|SaveGametoSlot (Variables|Default|GetSavesList) (Variables|Default|GetSaveListSlot)))

(fn ClearAutosaves
  (bind _saveslist (Variables|Default|GetSavesList))
  (bind _autosaves (Variables|/Game/Systems/BP_SavesListSave.BP_SavesListSave_C|GetAutosaves _saveslist))
  (for _array_element _autosaves
    (SaveGame|DeleteGameinSlot (CallFunction|GetSaveSlotName _array_element)))
  (Utilities|Array|Clear _autosaves)
  (SaveGame|SaveGametoSlot (Variables|Default|GetSavesList) (Variables|Default|GetSaveListSlot)))