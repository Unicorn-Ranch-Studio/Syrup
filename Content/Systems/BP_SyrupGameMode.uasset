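; BP_SyrupGameMode is the game mode for a turn-based tile game with plants and spreading trash.
; Phase events for plant growth, plant and trash effects, trash damage and trash spread each forward to TriggerPhaseEvent.
; BeginNight plays the LS_NightTime sequence with movement and look input disabled; its finish calls EndPlayerTurn after a delay.
; BeginPlay also briefly registers and removes a test tile label, apparently as debug code.
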(event Custom|Night%20Ended
  (Utilities|FlowControl|Delay 5.0)
  (Class|SyrupGameMode|EndPlayerTurn))

(event Custom|Plants%20Activate%20Active%20Effects
  (Class|SyrupGameMode|TriggerPhaseEvent "PlantActive"))

(event Custom|Trash%20Causes%20Damage
  (Class|SyrupGameMode|TriggerPhaseEvent "TrashDamage"))

(event Custom|Trash%20Acivates%20Active%20Effects
  (Class|SyrupGameMode|TriggerPhaseEvent "TrashActive"))

(event Custom|Trash%20Spreads
  (Class|SyrupGameMode|TriggerPhaseEvent "TrashSpread"))

(event Custom|Plants%20Grow
  (Class|SyrupGameMode|TriggerPhaseEvent "PlantsGrow"))

(event EventBeginPlay
  (bind _returnvalue (Sequencer|Player|CreateLevelSequencePlayer "/Game/Levels/LS_NightTime.LS_NightTime" (Utilities|Struct|MakeMovieSceneSequencePlaybackSettings false "(Value=0)" 1.0 0.0 false false true true false false false false)))
  (bind _output_get (Variables|Default|SetToNightSequencePlayer _returnvalue))
  (EventDispatchers|BindEventtoOnFinished _output_get (delegate Custom|Night%20Ended))
  (Utilities|FlowControl|Delay 2.0)
  (bind _returnvalue_2 (UserInterface|CreateWidget "/Game/UI/TileLabels/WBP_TestLabel.WBP_TestLabel_C"))
  (bind _output_get_2 (Variables|Default|SetNewVar_0 _returnvalue_2))
  (Class|SyrupGameMode|RegisterTileLabel _output_get_2 (Utilities|Struct|MakeIntPoint 1 10))
  (Utilities|FlowControl|Delay 2.0)
  (Class|SyrupGameMode|UnregisterTileLabel _output_get_2 (Utilities|Struct|MakeIntPoint 1 10)))

(event EventBeginNight
  (Sequencer|Player|Play (Variables|Default|GetToNightSequencePlayer) :!class /Script/MovieScene.MovieSceneSequencePlayer))

(fn ConstructionScript)