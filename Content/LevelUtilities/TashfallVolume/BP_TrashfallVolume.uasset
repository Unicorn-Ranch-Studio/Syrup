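; BP_TrashfallVolume is a level utility volume tied to a TrashType class; this graph only builds its visual marker.
; The construction script hashes three characters of the lowercased class name into a seed, giving each type a repeatable random hue.
; That hue tints a dynamic billboard icon material and a translucent Paper sprite.
; The sprite's Z scale copies Y, and the seed also offsets its translucency sorting.
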(fn ConstructionScript
  (bind _trashtype (Variables|Default|GetTrashType))
  (bind _papersprite (Variables|Default|GetPaperSprite))
  (bind _returnvalue (Utilities|GetClassDisplayName _trashtype))
  (bind _returnvalue_2 (Transformation|GetWorldScale _papersprite))
  (bind _returnvalue_3 (Utilities|String|ToLower _returnvalue))
  (bind _returnvalue_4 (Utilities|String|GetCharacterasNumber _returnvalue_3 5))
  (bind _returnvalue_5 (Utilities|String|GetCharacterasNumber _returnvalue_3 3))
  (bind _returnvalue_6 (Utilities|String|GetCharacterasNumber _returnvalue_3 4))
  (bind _returnvalue_7 (* _returnvalue_4 676))
  (bind _returnvalue_8 (* _returnvalue_6 26))
  (bind _returnvalue_9 (+ _returnvalue_5 _returnvalue_8 _returnvalue_7))
  (bind _returnvalue_10 (Math|Random|RandomFloatinRangefromStream 0.0 3.6e+02 (Math|Random|MakeRandomStream _returnvalue_9)))
  (bind _returnvalue_11 (Rendering|Material|CreateDynamicMaterialInstance (Variables|Default|GetMaterialBillboard) 0 "/Game/LevelUtilities/TashfallVolume/M_TrashfallVolume_Icon.M_TrashfallVolume_Icon" "None" :!class /Script/Engine.PrimitiveComponent))
  (Rendering|Material|SetVectorParameterValue _returnvalue_11 "color" (Class|KismetMathLibrary|HSVtoRGB _returnvalue_10 0.7 1.0 1.0) :!class /Script/Engine.MaterialInstanceDynamic)
  (Transformation|SetWorldScale3D _papersprite (Math|Vector|MakeVector (.x _returnvalue_2) (.y _returnvalue_2) (.y _returnvalue_2)))
  (Sprite|SetSpriteColor _papersprite (Class|KismetMathLibrary|HSVtoRGB _returnvalue_10 1.0 1.0 0.4))
  (Rendering|SetTranslucencySortDistanceOffset (Variables|Default|GetPaperSprite) (Math|Conversions|ToFloat(Integer) _returnvalue_9)))