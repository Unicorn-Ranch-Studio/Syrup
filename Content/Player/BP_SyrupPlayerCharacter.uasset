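; Player character for a turn-based, grid-based planting game, spending energy to pick up trash, sow plants and allocate selected resources.
; Number keys choose the plant, E picks up or sows, Q refills energy and ends the turn, R clears autosaves and opens a test level.
; Tick prints debug energy and plant lists, snaps the range previewer to the grid and recolors it by shape overlap to show placement validity.
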(event EventBeginPlay
  (|CallParentFunction)
  (CallFunction|SelectPlant))

(event EventTick
  (params (DeltaSeconds :type Float%20%28single-precision%29))
  (Development|PrintString (Utilities|String|Append "Energy: " (Utilities|String|ToString(Integer) (Variables|Default|GetPlayerEnergy)) "/" (Utilities|String|ToString(Integer) (.PlayerEnergy (Utilities|GetClassDefaults "BP_SyrupPlayerCharacter_C")))) true false "(R=1.000000,G=0.592295,B=0.000000,A=1.000000)" 2.0 "Player Energy")
  (for (_array_element _array_index) (Variables|Default|GetUnlockedPlantClasses)
    (Development|PrintString (Utilities|String|Append (Utilities|String|ToString(Integer) (+ _array_index 1)) " | " (Utilities|GetClassDisplayName _array_element)) true false (select (== _array_index (Variables|Default|GetSelectedPlant)) "(R=0.754167,G=0.135121,B=0.135121,A=1.000000)" "(R=0.166933,G=0.566667,B=0.000000,A=1.000000)") 2.0 (Utilities|String|StringToName (Utilities|GetClassDisplayName _array_element))))
  (Transformation|SetWorldTransform (Variables|Default|GetBP_RangePreviewer) (Math|Transform|ComposeTransforms (Math|Transform|MakeTransform (Math|Vector|MakeVector (/ (Class|GridLibrary|GetGridHeight) -3.0) 0.0 2.0) "0, 0, 0" "1.000000,1.000000,1.000000") (Class|GridLibrary|SnapWorldTransformtoGrid (Transformation|GetActorTransform))) false false)
  (bind _returnvalue (Class|GridLibrary|OverlapShape (Class|GridLibrary|TransformShape (Utilities|GetClassDefaults (Utilities|Array|Get(acopy) (Variables|Default|GetUnlockedPlantClasses) (Variables|Default|GetSelectedPlant))) (Class|GridLibrary|WorldTransformtoGridTransform (Transformation|GetActorTransform))) 0 "ECC_GameTraceChannel3"))
  (Rendering|Material|SetMaterial (Variables|Default|GetBP_RangePreviewer) 0 (select _returnvalue "/Game/Player/M_PlantPrevewer_Invalid.M_PlantPrevewer_Invalid" "/Game/Player/M_PlantPrevewer_Valid.M_PlantPrevewer_Valid")))

(event Input|KeyboardEvents|E
  (params (Key :type Key%20Structure))
  (bind _playerenergy (Variables|Default|GetPlayerEnergy))
  (:Pressed
    (bind _overlapingtile (Class|GridLibrary|OverlapGridLocation (Utilities|Struct|BreakGridTransform (Class|GridLibrary|WorldTransformtoGridTransform (Transformation|GetActorTransform))) 0 "ECC_WorldDynamic"))
    (bind _astrash (Utilities|Casting|CastToTrash _overlapingtile)
      (:then
        (Utilities|IsValid _astrash
          (:Is%20Valid
            (Class|Trash|PickUp _astrash _playerenergy))
          (:Is%20Not%20Valid
            (Class|Plant|SowPlant _playerenergy (Utilities|Array|Get(acopy) (Variables|Default|GetUnlockedPlantClasses) (Variables|Default|GetSelectedPlant)) (Transformation|GetActorTransform) :!label _label))))
      (:CastFailed
        (goto _label)))))

(event Input|KeyboardEvents|1
  (params (Key :type Key%20Structure))
  (:Pressed
    (CallFunction|SelectPlant)))

(event Input|KeyboardEvents|Q
  (params (Key :type Key%20Structure))
  (:Pressed
    (Variables|Default|SetPlayerEnergy (.PlayerEnergy (Utilities|GetClassDefaults "BP_SyrupPlayerCharacter_C")))
    (Variables|Default|SetSelectedResource 0)
    (Class|SyrupGameMode|EndPlayerTurn)))

(event Input|KeyboardEvents|5
  (params (Key :type Key%20Structure))
  (:Pressed
    (CallFunction|SelectPlant 4)))

(event Input|KeyboardEvents|2
  (params (Key :type Key%20Structure))
  (:Pressed
    (CallFunction|SelectPlant 1)))

(event Input|KeyboardEvents|3
  (params (Key :type Key%20Structure))
  (:Pressed
    (CallFunction|SelectPlant 2)))

(event Input|KeyboardEvents|4
  (params (Key :type Key%20Structure))
  (:Pressed
    (CallFunction|SelectPlant 3)))

(event Input|KeyboardEvents|R
  (params (Key :type Key%20Structure))
  (:Pressed
    (Default|ClearAutosaves (CallFunction|GetSyrupGameInstance))
    (Game|OpenLevel(byObjectReference) "/Game/Levels/L_Test_2.L_Test_2")))

(fn ConstructionScript)

(fn SelectResource
  (params (NewResource :type Resource%20Object%20Reference))
  (if (Class|SyrupGameMode|IsPlayerTurn)
    (Variables|Default|SetSelectedResource NewResource)
    (Default|CallNewResourceSelected NewResource)))

(fn GetSelectedResource
  (return (Variables|Default|GetSelectedResource)))

(fn AllocateResource
  (bind _playerenergy (Variables|Default|GetPlayerEnergy))
  (Math|Integer|CompareInt _playerenergy
    (:>
      (Math|Integer|DecrementInt _playerenergy
        (:%20%20
          (bind _selectedresource (Variables|Default|GetSelectedResource)
            (:then
              (bind _output_get (LocalVariables|SetOldSelectedResource _selectedresource))
              (Variables|Default|SetSelectedResource 0)
              (return _output_get))
            (:else)))))))

(fn SelectPlant
  (params (SelectedPlant :type Integer))
  (bind _output_get (Variables|Default|SetSelectedPlant SelectedPlant))
  (Default|UpdatePreview (Variables|Default|GetBP_RangePreviewer) (Utilities|GetClassDefaults (Utilities|Array|Get(acopy) (Variables|Default|GetUnlockedPlantClasses) _output_get))))